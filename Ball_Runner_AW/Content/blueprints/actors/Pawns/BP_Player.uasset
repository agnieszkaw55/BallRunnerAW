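; BP_Player is the player actor, a ball that rolls under player input.
; Two movement axis inputs apply scaled torque to the Kula component as an acceleration change, one axis around X and the other around Y.
; Any damage fades the camera out over a second, then reopens the current level, so a single hit restarts it.
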(event EventBeginPlay)

(event Collision|EventActorBeginOverlap
  (params (OtherActor :type Actor%20Object%20Reference)))

(event EventTick
  (params (DeltaSeconds :type Float%20%28single-precision%29)))

(event Game|Damage|EventAnyDamage
  (params (Damage :type Float%20%28single-precision%29) (DamageType :type Damage%20Type%20Object%20Reference) (InstigatedBy :type Controller%20Object%20Reference) (DamageCauser :type Actor%20Object%20Reference))
  (bind _returnvalue (Game|GetCurrentLevelName true))
  (CameraFades|StartCameraFade :self (Game|GetPlayerCameraManager 0) :ToAlpha 1.0 :Duration 1.0)
  (Utilities|FlowControl|Delay 1.0)
  (Game|OpenLevel(byName) (Utilities|String|StringToName _returnvalue)))

(event Input|AxisEvents|InputAxisMove_ForwardBack
  (params (AxisValue :type Float%20%28single-precision%29))
  (Class|PrimitiveComponent|AddTorqueinRadians (Variables|Default|Getkula) (Math|Vector|MakeVector 0.0 (* AxisValue (Variables|Default|GetMultiply)) 0.0) "None" true))

(event Input|AxisEvents|InputAxisMOve_RightLeft
  (params (AxisValue :type Float%20%28single-precision%29))
  (Class|PrimitiveComponent|AddTorqueinRadians (Variables|Default|Getkula) (Math|Vector|MakeVector (* AxisValue (Variables|Default|GetMultiply)) 0.0 0.0) "None" true))

(fn ConstructionScript)