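; BP_WinVolume is a volume that completes the level when the player overlaps it.
; On overlap it calls CompleteLevel only if CheckAnyCrystals finds at least one BP_Crystal actor still in the level.
; Completion looks up the current level name in the ordered LevelNames array, then opens the next entry or quits the game on the last one.
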(event EventBeginPlay)

(event EventTick
  (params (DeltaSeconds :type Float%20%28single-precision%29)))

(event Collision|EventActorBeginOverlap
  (params (OtherActor :type Actor%20Object%20Reference))
  (Utilities|PlayerIs OtherActor
    (:True
      (if (ArrayManagement|CheckAnyCrystals)
        (LevelManagement|CompleteLevel)))))

(fn ConstructionScript)

(fn CheckAnyCrystals
  (bind _outactors (Actor|GetAllActorsOfClass "/Game/blueprints/actors/actors/BP_Crystal.BP_Crystal_C"))
  (return (< 0 (Utilities|Array|Length _outactors))))

(fn CompleteLevel
  (if (LevelManagement|Isfinallevel (ArrayManagement|GetCurrentIndex))
    (Game|QuitGame 0 "Quit" false)
    (else
      (LevelManagement|LoadNextLevel))))

(fn GetCurrentIndex
  (bind _returnvalue (Game|GetCurrentLevelName true))
  (return (Utilities|Array|FindItem (Variables|Default|GetlevelNames) (Utilities|String|StringToName _returnvalue))))

(fn Isfinallevel
  (params (B :type Integer))
  (return (== (Utilities|Array|LastIndex (Variables|Default|GetlevelNames)) B)))

(fn LoadNextLevel
  (Game|OpenLevel(byName) (LevelManagement|GetNextLevelName)))

(fn GetNextLevelName
  (return (Utilities|Array|Get(acopy) (Variables|Default|GetlevelNames) (+ (ArrayManagement|GetCurrentIndex) 1))))